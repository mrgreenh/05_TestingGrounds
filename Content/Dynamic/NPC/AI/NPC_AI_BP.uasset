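; AI controller for a guard NPC that feeds perceived targets into its behavior tree.
; On BeginPlay it initializes the PatrolData blackboard and runs the GuardBehavior tree.
; AI Perception updates ignore actors tagged "Enemy".
; For any other actor, a successful sense stores it in the blackboard's Enemy key, and a failed sense clears that key.
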(event OnTargetPerceptionUpdated(AIPerception)
  (params (Actor :type Actor%20Object%20Reference) (Stimulus :type AI%20Stimulus%20Structure))
  (bind _enemy (Variables|Default|GetEnemy))
  (bind _blackboardcomponent (Variables|Default|GetBlackboardComponent))
  (if (not (Actor|ActorHasTag Actor "Enemy"))
    (if (.bSuccessfullySensed (Utilities|Struct|BreakAIStimulus Stimulus))
      (AI|Components|Blackboard|SetValueasObject _blackboardcomponent _enemy Actor)
      (else
        (AI|Components|Blackboard|ClearValue _blackboardcomponent _enemy)))))

(event EventBeginPlay
  (bind _blackboardcomponent (Class|AIController|UseBlackboard "/Game/Dynamic/NPC/AI/PatrolData.PatrolData"))
  (AI|RunBehaviorTree "/Game/Dynamic/NPC/AI/GuardBehavior.GuardBehavior")
  (Variables|Default|SetBlackboardComponent _blackboardcomponent))

(fn ConstructionScript)